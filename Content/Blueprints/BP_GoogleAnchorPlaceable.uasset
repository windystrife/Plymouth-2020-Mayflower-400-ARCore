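; Placeable AR prop that carries a Google ARCore anchor actor as a child actor and shows a randomly chosen cone, sphere or cylinder mesh.
; The construction script picks the mesh.
; On BeginPlay it caches the anchor, then, if that cast succeeds or not, plays a timeline that animates the mesh's drop and scale.
; HandleVisibility and GetIfStoppedTracking are unfinished stubs with no effect.
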(event `self.ReceiveBeginPlay`
  (bind _staticmesh (`self.StaticMesh`))
  (`|ExecutionSequence`
    (:`then_0`
      ;[1 1 1] Set Up Google Anchor Child Actor.
      (bind _asgoogle_arcore_anchor_actor (cast `GoogleARCoreAnchorActor` (`ChildActorComponent.ChildActor` (`self.ChildActor`))))
      (set `self.AnchorActor` _asgoogle_arcore_anchor_actor))
    (:`then_1`
      ;[1 1 1] Do Drop Animation
      (bind (_direction _fall _scaleanim) (`Timeline|Intro Anim` :!via `PlayFromStart`)
        (:`Update`
          (`SceneComponent.K2_SetRelativeLocation` _staticmesh _fall false true)
          (`SceneComponent.SetRelativeScale3D` _staticmesh _scaleanim))))))

(fn `GetIfStoppedTracking`
  (returns (ActorOrPlaneStoppedTracking :type Boolean))
  (return false))

(fn `HandleVisibility`
  (params (Delta :type "Float (double-precision)"))
  (if (`self.GetIfStoppedTracking`)
    _))

(fn `UserConstructionScript`
  (switch `int` (`KismetMathLibrary.RandomInteger` 3)
    (:`0`
      (`StaticMeshComponent.SetStaticMesh` (`self.StaticMesh`) "/Engine/BasicShapes/Cone.Cone"))
    (:`1`
      (`StaticMeshComponent.SetStaticMesh` (`self.StaticMesh`) "/Engine/BasicShapes/Sphere.Sphere"))
    (:`2`
      (`StaticMeshComponent.SetStaticMesh` (`self.StaticMesh`) "/Engine/BasicShapes/Cylinder.Cylinder"))))